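; BP_PerspectiveViewPlates is a trigger plate that switches the player's view to a shared perspective camera in UnblockMe.
; On BeginPlay it caches the BP_CameraPerspective actor.
; Any Box overlap moves that camera to the plate's root X and Y, keeping the camera component's height.
; If the overlapping actor is BP_UnblockMeCharacter, its PC_PlayerController4UnblockMe then blends the view target to that camera.
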(event `self.ReceiveBeginPlay`
  (bind _returnvalue (`GameplayStatics.GetActorOfClass` "/Game/UnblockMe/BP_CameraPerspective.BP_CameraPerspective_C"))
  (set `self.Camera` _returnvalue))

(event `self.Box.OnComponentBeginOverlap`
  (params (OverlappedComponent :type "PrimitiveComponent Object Reference") (OtherActor :type "Actor Object Reference") (OtherComp :type "PrimitiveComponent Object Reference") (OtherBodyIndex :type Integer) (bFromSweep :type Boolean) (SweepResult :type "HitResult Structure (by ref)"))
  (bind _camera (`self.Camera`))
  (bind (_returnvalue_x _returnvalue_y) (`KismetMathLibrary.BreakVector` (`SceneComponent.K2_GetComponentLocation` (`self.DefaultSceneRoot`))))
  (bind (_returnvalue_x_2 _returnvalue_y_2 _returnvalue_z) (`KismetMathLibrary.BreakVector` (`SceneComponent.K2_GetComponentLocation` (`CameraActor.CameraComponent` _camera))))
  (`self.K2_SetActorLocation` _camera (`KismetMathLibrary.MakeVector` _returnvalue_x _returnvalue_y _returnvalue_z) false false)
  (bind _asbp_unblock_me_character (cast `/Game/UnblockMe/BP_UnblockMeCharacter` OtherActor))
  (if (`KismetSystemLibrary.IsValid` _asbp_unblock_me_character)
    (bind _aspc_player_controller_4unblock_me (cast `/Game/UnblockMe/PC_PlayerController4UnblockMe` (`Pawn.GetController` _asbp_unblock_me_character)))
    (if (`KismetSystemLibrary.IsValid` _aspc_player_controller_4unblock_me)
      (`PlayerController.SetViewTargetWithBlend` _aspc_player_controller_4unblock_me (`self.Camera`) 1.0 "VTBlend_Linear" 0.0 false))))

(fn `UserConstructionScript`)