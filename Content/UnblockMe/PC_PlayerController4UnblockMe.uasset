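; Player controller for an Unblock Me puzzle that shows the mouse cursor and lets the player move blocks.
; Left click stores the "Moveable"-tagged actor under the cursor in ObjectInHand, and middle click clears it.
; Arrow keys shift it in fixed X/Y steps with swept moves, applying an unswept opposite step if the move returns false.
; E makes a swept +X step without validity or failure checks.
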(event `Key|MiddleMouseButton`
  (params (Key :type "Key Structure"))
  ;[1 1 1] Clear Selection
  (:`Pressed`
    (if (`KismetSystemLibrary.IsValid` (`self.ObjectInHand`))
      (set `self.ObjectInHand` (`self.NULL ACTOR`)))))

(event `Key|LeftMouseButton`
  (params (Key :type "Key Structure"))
  (bind (_bblockinghit _binitialoverlap _time _distance _location _impactpoint _normal _impactnormal _physmat _hitactor) (`GameplayStatics.BreakHitResult` (`self.GetHitResultUnderCursorByChannel` "TraceTypeQuery1")))
  ;[1 1 1] Select the object
  (:`Pressed`
    (if (`self.ActorHasTag` _hitactor "Moveable")
      (set `self.ObjectInHand` _hitactor))))

(event `Key|E`
  (params (Key :type "Key Structure"))
  (bind _objectinhand (`self.ObjectInHand`))
  (bind (_returnvalue_x _returnvalue_y _returnvalue_z) (`KismetMathLibrary.BreakVector` (`self.K2_GetActorLocation` _objectinhand)))
  (:`Pressed`
    (`self.K2_SetActorLocation` _objectinhand (`KismetMathLibrary.MakeVector` (+ _returnvalue_x 200.0) _returnvalue_y _returnvalue_z) true false)))

(event `self.ReceiveBeginPlay`
  (set `self.bShowMouseCursor` true) ; toggle  mouse cursor
)

(event `self.ReceiveTick`
  (params (DeltaSeconds :type "Float (single-precision)")))

(event `Key|Up`
  (params (Key :type "Key Structure"))
  (bind _objectinhand (`self.ObjectInHand`))
  (bind _objectinhand_2 (`self.ObjectInHand`))
  (bind (_returnvalue_x _returnvalue_y _returnvalue_z) (`KismetMathLibrary.BreakVector` (`self.K2_GetActorLocation` _objectinhand)))
  (bind (_returnvalue_x_2 _returnvalue_y_2 _returnvalue_z_2) (`KismetMathLibrary.BreakVector` (`self.K2_GetActorLocation` _objectinhand_2)))
  (:`Pressed`
    (if (`KismetSystemLibrary.IsValid` (`self.ObjectInHand`))
      (bind (_sweephitresult _returnvalue) (`self.K2_SetActorLocation` _objectinhand (`KismetMathLibrary.MakeVector` (- _returnvalue_x 200.0) _returnvalue_y _returnvalue_z) true false))
      (if (not _returnvalue)
        (`self.K2_SetActorLocation` _objectinhand_2 (`KismetMathLibrary.MakeVector` (+ _returnvalue_x_2 200.0) _returnvalue_y_2 _returnvalue_z_2) false false))
      (else
        (`KismetSystemLibrary.PrintString` "Object not selected" :!label _label)))))

(event `Key|Down`
  (params (Key :type "Key Structure"))
  (bind _objectinhand (`self.ObjectInHand`))
  (bind _objectinhand_2 (`self.ObjectInHand`))
  (bind (_returnvalue_x _returnvalue_y _returnvalue_z) (`KismetMathLibrary.BreakVector` (`self.K2_GetActorLocation` _objectinhand)))
  (bind (_returnvalue_x_2 _returnvalue_y_2 _returnvalue_z_2) (`KismetMathLibrary.BreakVector` (`self.K2_GetActorLocation` _objectinhand_2)))
  (:`Pressed`
    (if (`KismetSystemLibrary.IsValid` (`self.ObjectInHand`))
      (bind (_sweephitresult _returnvalue) (`self.K2_SetActorLocation` _objectinhand (`KismetMathLibrary.MakeVector` (+ _returnvalue_x 200.0) _returnvalue_y _returnvalue_z) true false))
      (if (not _returnvalue)
        (`self.K2_SetActorLocation` _objectinhand_2 (`KismetMathLibrary.MakeVector` (- _returnvalue_x_2 200.0) _returnvalue_y_2 _returnvalue_z_2) false false))
      (else
        (goto _label)))))

(event `Key|Left`
  (params (Key :type "Key Structure"))
  (bind _objectinhand (`self.ObjectInHand`))
  (bind _objectinhand_2 (`self.ObjectInHand`))
  (bind (_returnvalue_x _returnvalue_y _returnvalue_z) (`KismetMathLibrary.BreakVector` (`self.K2_GetActorLocation` _objectinhand_2)))
  (bind (_returnvalue_x_2 _returnvalue_y_2 _returnvalue_z_2) (`KismetMathLibrary.BreakVector` (`self.K2_GetActorLocation` _objectinhand)))
  (:`Pressed`
    (if (`KismetSystemLibrary.IsValid` (`self.ObjectInHand`))
      (bind (_sweephitresult _returnvalue) (`self.K2_SetActorLocation` _objectinhand (`KismetMathLibrary.MakeVector` _returnvalue_x_2 (+ _returnvalue_y_2 200.0) _returnvalue_z_2) true false))
      (if (not _returnvalue)
        (`self.K2_SetActorLocation` _objectinhand_2 (`KismetMathLibrary.MakeVector` _returnvalue_x (- _returnvalue_y 200.0) _returnvalue_z) false false))
      (else
        (goto _label)))))

(event `Key|Right`
  (params (Key :type "Key Structure"))
  (bind _objectinhand (`self.ObjectInHand`))
  (bind _objectinhand_2 (`self.ObjectInHand`))
  (bind (_returnvalue_x _returnvalue_y _returnvalue_z) (`KismetMathLibrary.BreakVector` (`self.K2_GetActorLocation` _objectinhand_2)))
  (bind (_returnvalue_x_2 _returnvalue_y_2 _returnvalue_z_2) (`KismetMathLibrary.BreakVector` (`self.K2_GetActorLocation` _objectinhand)))
  (:`Pressed`
    (if (`KismetSystemLibrary.IsValid` (`self.ObjectInHand`))
      (bind (_sweephitresult _returnvalue) (`self.K2_SetActorLocation` _objectinhand (`KismetMathLibrary.MakeVector` _returnvalue_x_2 (- _returnvalue_y_2 200.0) _returnvalue_z_2) true false))
      (if (not _returnvalue)
        (`self.K2_SetActorLocation` _objectinhand_2 (`KismetMathLibrary.MakeVector` _returnvalue_x (+ _returnvalue_y 200.0) _returnvalue_z) false false))
      (else
        (goto _label)))))

(fn `UserConstructionScript`)