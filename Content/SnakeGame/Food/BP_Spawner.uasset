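; BP_Spawner is the food spawner for the snake game, scattering apples and grapes across an area.
; Tick runs through a 3-second Delay, so roughly every three seconds a random bool picks BP_Apple or BP_Grapes.
; The chosen food spawns at a random X and Y within the Box component's scaled extent around the actor, at the actor's Z height.
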(event `self.ReceiveTick`
  (params (DeltaSeconds :type "Float (single-precision)"))
  (bind (_returnvalue_x _returnvalue_y _returnvalue_z) (`KismetMathLibrary.BreakVector` (`self.K2_GetActorLocation`)))
  (bind (_returnvalue_x_2 _returnvalue_y_2) (`KismetMathLibrary.BreakVector` (`BoxComponent.GetScaledBoxExtent` (`self.Box`))))
  (bind _returnvalue (`KismetMathLibrary.MakeVector` (+ _returnvalue_x (`KismetMathLibrary.RandomFloatInRange` (* _returnvalue_x_2 -1.0) _returnvalue_x_2)) (+ _returnvalue_y (`KismetMathLibrary.RandomFloatInRange` (* _returnvalue_y_2 -1.0) _returnvalue_y_2)) _returnvalue_z))
  (`KismetSystemLibrary.Delay` 3.0)
  (if (`KismetMathLibrary.RandomBool`)
    (`|SpawnActorFromClass` "/Game/SnakeGame/Food/Apple/BP_Apple.BP_Apple_C" (`KismetMathLibrary.MakeTransform` _returnvalue) "Undefined" "MultiplyWithRoot" null null)
    (else
      (`|SpawnActorFromClass` "/Game/SnakeGame/Food/Grapes/BP_Grapes.BP_Grapes_C" (`KismetMathLibrary.MakeTransform` _returnvalue) "Undefined" "MultiplyWithRoot" null null))))

(fn `UserConstructionScript`)