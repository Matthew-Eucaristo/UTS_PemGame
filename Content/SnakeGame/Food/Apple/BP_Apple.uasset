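; BP_Apple is a food pickup for the snake game that grows the player's snake by one body segment when consumed.
; Its Consume event casts the player character to BP_Snake and adds an ISMBody instance at the last segment's local transform, then destroys the apple through a short lifespan.
; IsFood always returns true to identify it as food, and Tick only calls the parent.
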(event `self.ReceiveTick`
  (params (DeltaSeconds :type "Float (single-precision)"))
  (`parent.ReceiveTick` 0.0))

(event `/Game/SnakeGame/Food/BI_Food.Consume`
  (bind _asbp_snake (cast `/Game/SnakeGame/Snake/BP_Snake` (`GameplayStatics.GetPlayerCharacter` 0)))
  (if (`KismetSystemLibrary.IsValid` _asbp_snake)
    (bind _ism_body (`/Game/SnakeGame/Snake/BP_Snake.ISM_Body` _asbp_snake))
    (`InstancedStaticMeshComponent.AddInstance` (`/Game/SnakeGame/Snake/BP_Snake.ISM_Body` _asbp_snake) (`InstancedStaticMeshComponent.GetInstanceTransform` _ism_body (- (`InstancedStaticMeshComponent.GetInstanceCount` _ism_body) 1) false) false)
    (`self.SetLifeSpan` 0.1)))

(fn `Is Food`
  (returns (`Is Food` :type Boolean))
  (return true))

(fn `UserConstructionScript`)