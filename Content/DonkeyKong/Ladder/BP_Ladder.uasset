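; BP_Ladder is a ladder in the Donkey Kong game that tells BP_DonkeyCharacter when it can climb.
; Beginning or ending overlap with the Range component sets the character's CanClimb flag on or off.
; Both events also write the Arrow component's world location to the character's LadderTopPosition, so the arrow marks the top of the ladder.
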(event `self. Range.OnComponentBeginOverlap`
  (params (OverlappedComponent :type "PrimitiveComponent Object Reference") (OtherActor :type "Actor Object Reference") (OtherComp :type "PrimitiveComponent Object Reference") (OtherBodyIndex :type Integer) (bFromSweep :type Boolean) (SweepResult :type "HitResult Structure (by ref)"))
  (bind _asbp_donkey_character (cast `/Game/DonkeyKong/BP_DonkeyCharacter` OtherActor))
  (if (`KismetSystemLibrary.IsValid` _asbp_donkey_character)
    (set `/Game/DonkeyKong/BP_DonkeyCharacter.Can Climb` true _asbp_donkey_character)
    (set `/Game/DonkeyKong/BP_DonkeyCharacter.Ladder Top Position` (`SceneComponent.K2_GetComponentLocation` (`self.Arrow`)) _asbp_donkey_character :!label _label)))

(event `self. Range.OnComponentEndOverlap`
  (params (OverlappedComponent :type "PrimitiveComponent Object Reference") (OtherActor :type "Actor Object Reference") (OtherComp :type "PrimitiveComponent Object Reference") (OtherBodyIndex :type Integer))
  (bind _asbp_donkey_character (cast `/Game/DonkeyKong/BP_DonkeyCharacter` OtherActor))
  (if (`KismetSystemLibrary.IsValid` _asbp_donkey_character)
    (set `/Game/DonkeyKong/BP_DonkeyCharacter.Can Climb` false _asbp_donkey_character)
    (goto _label)))

(fn `UserConstructionScript`)