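; BP_ChangeViewTrigger is a Donkey Kong trigger volume that starts gameplay when BP_DonkeyCharacter overlaps its box.
; It blends the player controller's view to the level's BP_FarCamera over a configurable Blend time.
; It then teleports the character to the BP_StartLocation arrow's transform and sets GameStarted on the character, finding both camera and start point by class lookup.
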(event `self.Box.OnComponentBeginOverlap`
  (params (OverlappedComponent :type "PrimitiveComponent Object Reference") (OtherActor :type "Actor Object Reference") (OtherComp :type "PrimitiveComponent Object Reference") (OtherBodyIndex :type Integer) (bFromSweep :type Boolean) (SweepResult :type "HitResult Structure (by ref)"))
  ;[1 1 1] Change View
  (bind _asbp_donkey_character (cast `/Game/DonkeyKong/BP_DonkeyCharacter` OtherActor))
  (if (`KismetSystemLibrary.IsValid` _asbp_donkey_character)
    (bind _asplayer_controller (cast `PlayerController` (`Pawn.GetController` _asbp_donkey_character)))
    (if (`KismetSystemLibrary.IsValid` _asplayer_controller)
      (bind _returnvalue (`GameplayStatics.GetActorOfClass` "/Game/DonkeyKong/BP_FarCamera.BP_FarCamera_C"))
      (`PlayerController.SetViewTargetWithBlend` _asplayer_controller _returnvalue (`self.Blend`) "VTBlend_Linear" 0.0 false)
      ;[1 1 1] Teleport the character
      (bind _returnvalue_2 (`GameplayStatics.GetActorOfClass` "/Game/DonkeyKong/BP_StartLocation.BP_StartLocation_C"))
      (if (`KismetSystemLibrary.IsValid` _returnvalue_2)
        (bind _arrow (`/Game/DonkeyKong/BP_StartLocation.Arrow` _returnvalue_2))
        (`self.K2_SetActorLocationAndRotation` _asbp_donkey_character (`SceneComponent.K2_GetComponentLocation` _arrow) (`SceneComponent.K2_GetComponentRotation` _arrow) false false)
        (set `/Game/DonkeyKong/BP_DonkeyCharacter.GameStarted` true _asbp_donkey_character) ; change the state that the game is now started
      ))))

(fn `UserConstructionScript`)