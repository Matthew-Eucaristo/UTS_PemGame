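; BP_Peach is the Princess Peach goal actor that triggers the win condition in a Donkey Kong game.
; When a BP_DonkeyCharacter overlaps its WinningRange component, it prints a win message, creates a win widget on the viewport and shows the mouse cursor.
; It also finds the BP_Donkey actor in the level and sets its Donkey component's animation to a backward death reaction.
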(event `self.WinningRange.OnComponentBeginOverlap`
  (params (OverlappedComponent :type "PrimitiveComponent Object Reference") (OtherActor :type "Actor Object Reference") (OtherComp :type "PrimitiveComponent Object Reference") (OtherBodyIndex :type Integer) (bFromSweep :type Boolean) (SweepResult :type "HitResult Structure (by ref)"))
  ;[1 1 1] Win condition
  (bind _asbp_donkey_character (cast `/Game/DonkeyKong/BP_DonkeyCharacter` OtherActor))
  (if (`KismetSystemLibrary.IsValid` _asbp_donkey_character)
    (`KismetSystemLibrary.PrintString` "You Win")
    (bind _returnvalue (`GameplayStatics.GetActorOfClass` "/Game/DonkeyKong/Donkey/BP_Donkey.BP_Donkey_C"))
    (`SkeletalMeshComponent.SetAnimation` (`/Game/DonkeyKong/Donkey/BP_Donkey.Donkey` _returnvalue) "/Game/DonkeyKong/Donkey/Standing_React_Death_Backward_Anim.Standing_React_Death_Backward_Anim")
    (bind _returnvalue_2 (`|CreateWidget` "/Game/UI/UI_Win.UI_Win_C"))
    (`UserWidget.AddToViewport` _returnvalue_2 0)
    (set `PlayerController.bShowMouseCursor` true (`GameplayStatics.GetPlayerController` 0))))

(fn `UserConstructionScript`)